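; Mothership shot projectile that hits the Hero on contact.
; When its Capsule overlaps a Hero, it destroys itself and calls HitCheck on that Hero; other actors are ignored.
; RaycastLocation1 traces along +X at a fixed world Y with persistent debug drawing and returns the trace end, not the impact point.
; RaycastLocation2 is an unfinished stub, and neither raycast function is called within this Blueprint.
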(event OnComponentBeginOverlap(Capsule)
  (params (OverlappedComponent :type Primitive%20Component%20Object%20Reference) (OtherActor :type Actor%20Object%20Reference) (OtherComp :type Primitive%20Component%20Object%20Reference) (OtherBodyIndex :type Integer) (bFromSweep :type Boolean) (SweepResult :type Hit%20Result%20Structure%20%28by%20ref%29))
  (bind _ashero (Utilities|Casting|CastToHero OtherActor))
  (Actor|DestroyActor)
  (Default|Hit-Check _ashero))

(event EventBeginPlay)

(event Collision|EventActorBeginOverlap
  (params (OtherActor :type Actor%20Object%20Reference)))

(event EventTick
  (params (DeltaSeconds :type Float%20%28single-precision%29)))

(fn ConstructionScript)

(fn RaycastLocation1
  (bind _defaultsceneroot (Variables|Default|GetDefaultSceneRoot))
  (bind _returnvalue (Transformation|GetWorldTransform _defaultsceneroot))
  (bind _returnvalue_2 (+ (.location _returnvalue) "660.000000,0,0"))
  (bind _outhit (Collision|LineTraceByChannel (.location _returnvalue) (Math|Vector|MakeVector (.x _returnvalue_2) -4e+01 (.z _returnvalue_2)) "TraceTypeQuery1" false 0 "Persistent"))
  (return (.TraceEnd (Collision|BreakHitResult _outhit))))

(fn RaycastLocation2
  (Collision|LineTraceByChannel "0, 0, 0" "0, 0, 0" "TraceTypeQuery1" false 0 "None"))