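; Hero bullet projectile that damages enemy invaders and the Mothership on contact.
; On spawn it deactivates its Box component and reactivates it after a short delay.
; A Box overlap with a Frontline_Invader destroys the bullet and calls ShipDies with that invader's ShipID.
; An overlap with the Mothership destroys the bullet and decrements its HP, while other actors are ignored.
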(event OnComponentBeginOverlap(Box)
  (params (OverlappedComponent :type Primitive%20Component%20Object%20Reference) (OtherActor :type Actor%20Object%20Reference) (OtherComp :type Primitive%20Component%20Object%20Reference) (OtherBodyIndex :type Integer) (bFromSweep :type Boolean) (SweepResult :type Hit%20Result%20Structure%20%28by%20ref%29))
  (bind _asfrontline_invader (Utilities|Casting|CastToFrontline_Invader OtherActor)
    (:then
      (Actor|DestroyActor)
      (Default|ShipDies _asfrontline_invader (Variables|/Game/Blueprints/Invaders/Basic_Invader/Frontline_Invader.Frontline_Invader_C|GetShip_ID _asfrontline_invader)))
    (:CastFailed
      (bind _asmothership (Utilities|Casting|CastToMothership OtherActor))
      (Actor|DestroyActor)
      (Variables|/Game/Blueprints/Invaders/Invader_Mothership(Optional))/Mothership.Mothership_C|SetHP _asmothership (- (Variables|/Game/Blueprints/Invaders/Invader_Mothership(Optional))/Mothership.Mothership_C|GetHP _asmothership) 1)))))

(event Collision|EventActorBeginOverlap
  (params (OtherActor :type Actor%20Object%20Reference)))

(event EventTick
  (params (DeltaSeconds :type Float%20%28single-precision%29)))

(event EventBeginPlay
  (bind _box (Variables|Default|GetBox))
  (Components|Activation|Deactivate _box)
  (Utilities|FlowControl|Delay 0.2)
  (Components|Activation|Activate _box true))

(fn ConstructionScript)